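; BP_RGideon is a Gideon Blueprint that binds debug-style keys and animates the quest side panel on the main UI widget.
; G adds the BP_QuesTwo quest through QuestManager, P calls UnEquipItem and T calls TEST01.
; PlaySideOutAnimation toggles WBP_Mian's slide animation when quests exist, reversing it mid-play and tracking state in OutSide.
; PlayAddNewQuestAnimation plays the slide backwards and clears OutSide if it was set.
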(event EventBeginPlay)

(event Collision|EventActorBeginOverlap
  (params (OtherActor :type Actor%20Object%20Reference)))

(event EventTick
  (params (DeltaSeconds :type Float%20%28single-precision%29)))

(event EventPlaySideOutAnimation
  (bind _aswbp_mian (Utilities|Casting|CastToWBP_Mian (Variables|Default|GetMainUserWidget)))
  (bind _output_get (Variables|Default|SetWBP_Mian _aswbp_mian))
  (if (>= (Utilities|Array|Length (Variables|/Script/RPGProject.MainUserWidget|GetQuestWidgets (Variables|Default|GetWBP_Mian))) 1)
    (if (Class|UserWidget|IsAnimationPlaying (Variables|Default|GetWBP_Mian) (Variables|/Game/Blueprints/UI/WBP_Mian.WBP_Mian_C|GetSideOutAnimation (Variables|Default|GetWBP_Mian)))
      (Class|UserWidget|ReverseAnimation (Variables|Default|GetWBP_Mian) (Variables|/Game/Blueprints/UI/WBP_Mian.WBP_Mian_C|GetSideOutAnimation (Variables|Default|GetWBP_Mian)))
      (else
        (Components|Animation|PlayAnimation _output_get (Variables|/Game/Blueprints/UI/WBP_Mian.WBP_Mian_C|GetSideOutAnimation (Variables|Default|GetWBP_Mian)) 0.0 1 (select (Variables|/Script/RPGProject.MainUserWidget|GetbOutSide _output_get) "Reverse" "Forward")
          (:then
            _))))
    (Variables|/Script/RPGProject.MainUserWidget|SetbOutSide (Variables|Default|GetWBP_Mian) (not (Variables|/Script/RPGProject.MainUserWidget|GetbOutSide (Variables|Default|GetWBP_Mian))))))

(event EventPlayAddNewQuestAnimation
  (bind _mainuserwidget (Variables|Default|GetMainUserWidget))
  (bind _aswbp_mian (Utilities|Casting|CastToWBP_Mian _mainuserwidget))
  (if (Variables|/Script/RPGProject.MainUserWidget|GetbOutSide _aswbp_mian)
    (Components|Animation|PlayAnimation _mainuserwidget (Variables|/Game/Blueprints/UI/WBP_Mian.WBP_Mian_C|GetSideOutAnimation _aswbp_mian) 0.0 1 "Reverse"
      (:then
        (Variables|/Script/RPGProject.MainUserWidget|SetbOutSide _mainuserwidget false)))))

(event Input|KeyboardEvents|G
  (params (Key :type Key%20Structure :default "None"))
  (:Pressed
    (Class|QuestManager|AddNewQuset (Variables|Default|GetQuestManager) "/Game/Blueprints/Quest/BP_QuesTwo.BP_QuesTwo_C")))

(event Input|KeyboardEvents|P
  (params (Key :type Key%20Structure :default "None"))
  (:Pressed
    (Class|RBaseCharacter|UnEquipItem)))

(event Input|KeyboardEvents|T
  (params (Key :type Key%20Structure :default "None"))
  (:Pressed
    (Class|RBaseCharacter|TEST01)))

(fn ConstructionScript)